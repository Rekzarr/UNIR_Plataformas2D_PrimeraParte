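; Flying enemy that patrols between waypoints, shoots at the player and dies when bullet hits deplete its health.
; Tick drives swept movement toward each patrol point in turn, looping through the array by modulo index.
; A looping fire-rate timer checks range to the cached player, turns the enemy and spawns an aimed actor at its arrow.
; Overlapping BP_Bullet actors reduce health, print debug text and are destroyed.
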(event Custom|Disparo
  (CallFunction|Fire))

(event EventBeginPlay
  (bind _asbp_third_person_character (Utilities|Casting|CastToBP_ThirdPersonCharacter (Game|GetPlayerCharacter 0)))
  (Variables|Default|SetPlayerReference _asbp_third_person_character)
  (Utilities|Time|SetTimerbyEvent (delegate Custom|Disparo) (Variables|Default|GetFireRate) true))

(event Collision|EventActorBeginOverlap
  (params (OtherActor :type Actor%20Object%20Reference))
  (bind _asbp_bullet (Utilities|Casting|CastToBP_Bullet OtherActor))
  (Variables|Default|SetVida (- (Variables|Default|GetVida) 2e+01))
  (Development|PrintText "Hello")
  (Actor|DestroyActor _asbp_bullet)
  (if (<= (Variables|Default|GetVida) 0.0)
    (Actor|DestroyActor)))

(event EventTick
  (params (DeltaSeconds :type Float%20%28single-precision%29))
  (CallFunction|MovimientoPatrulla DeltaSeconds))

(fn ConstructionScript)

(fn MovimientoPatrulla
  (params (B :type Float%20%28single-precision%29))
  (bind _returnvalue (Transformation|GetActorLocation))
  (bind _puntospatrulla (Variables|Default|GetPuntosPatrulla))
  (bind _returnvalue_2 (Utilities|Array|Length _puntospatrulla))
  (if (> _returnvalue_2 0)
    (Transformation|AddActorWorldOffset (* (Math|Vector|Normalize (- (Transformation|GetActorLocation (Utilities|Array|Get(acopy) _puntospatrulla (Math|Integer|%(Integer) (Variables|Default|GetCurrentPatrol) _returnvalue_2))) _returnvalue)) (* (Variables|Default|GetPatrolSpeed) B)) true)
    (if (< (Math|Vector|Distance(Vector) (Transformation|GetActorLocation (Utilities|Array|Get(acopy) _puntospatrulla (Math|Integer|%(Integer) (Variables|Default|GetCurrentPatrol) _returnvalue_2))) _returnvalue) (Variables|Default|GetPatrolTolerance))
      (Variables|Default|SetCurrentPatrol (+ (Variables|Default|GetCurrentPatrol) 1)))))

(fn Fire
  (bind _returnvalue (Transformation|GetActorLocation))
  (bind _playerreference (Variables|Default|GetPlayerReference))
  (bind _returnvalue_2 (Transformation|GetActorLocation _playerreference))
  (bind _returnvalue_3 (Math|Rotator|FindLookatRotation _returnvalue _returnvalue_2))
  (if (< (Math|Vector|Distance(Vector) _returnvalue _returnvalue_2) (Variables|Default|GetFireRange))
    (Transformation|SetActorRotation _returnvalue_3)
    (Game|SpawnActorfromClass "/Game/00_Plataformas_2D/Weapons/BP_BulletEnemy.BP_BulletEnemy_C" (Math|Transform|MakeTransform (Transformation|GetWorldLocation (Variables|Default|GetArrow)) _returnvalue_3 "1.000000,1.000000,1.000000") "Undefined" "MultiplyWithRoot" 0 0)))