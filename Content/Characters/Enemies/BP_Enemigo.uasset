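; BP_Enemigo is an enemy that takes damage from bullets and drops a power-up when killed.
; On overlap with a BP_Bullet, it subtracts a fixed amount from its Vida health, prints the new value and destroys the bullet.
; When Vida reaches zero, it destroys itself and spawns a BP_PowerUp slightly above its location.
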(event EventBeginPlay)

(event Collision|EventActorBeginOverlap
  (params (OtherActor :type Actor%20Object%20Reference))
  (bind _asbp_bullet (Utilities|Casting|CastToBP_Bullet OtherActor))
  (Variables|Default|SetVida (- (Variables|Default|GetVida) 2e+01))
  (Development|PrintText (Utilities|Text|ToText(Float) (Variables|Default|GetVida) "HalfToEven"))
  (Actor|DestroyActor _asbp_bullet)
  (if (<= (Variables|Default|GetVida) 0.0)
    (Actor|DestroyActor)
    (Game|SpawnActorfromClass "/Game/ThirdPerson/Blueprints/BP_PowerUp.BP_PowerUp_C" (Math|Conversions|ToTransform(Vector) (+ (Transformation|GetActorLocation) "0.000000,0.000000,50.000000")) "Undefined" "MultiplyWithRoot" 0 0)))

(event EventTick
  (params (DeltaSeconds :type Float%20%28single-precision%29)))

(fn ConstructionScript)